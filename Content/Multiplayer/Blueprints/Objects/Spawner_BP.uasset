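; Pickup spawner for a multiplayer game that presents one item, chosen by SpawnType: health, rifle, shotgun, or ammo for either gun.
; The construction script gathers all candidate child actor components into an array, keeps the matching one as ChosenActor and destroys the rest.
; At BeginPlay a fast looping timer starts, continuously spinning Cylinder1 in yaw via FInterpTo.
; The file contains no pickup or respawn logic.
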(event `self.ReceiveBeginPlay`
  (`KismetSystemLibrary.K2_SetTimerDelegate` (delegate `PlayFromStart`) 0.01 true))

(event `PlayFromStart`
  (bind _cylinder1 (`self.Cylinder1`))
  (bind (_relativerotation_roll _relativerotation_pitch _relativerotation_yaw) (`KismetMathLibrary.BreakRotator` (`SceneComponent.RelativeRotation` _cylinder1)))
  (`SceneComponent.K2_SetRelativeRotation` _cylinder1 (`KismetMathLibrary.MakeRotator` 0.0 0.0 (`KismetMathLibrary.FInterpTo` _relativerotation_yaw (+ _relativerotation_yaw 3.0) (`GameplayStatics.GetWorldDeltaSeconds`) 20.0)) false false))

(fn `RemoveOtherComponents`
  (params (Component :type "Object Object Reference"))
  (for _array_element (`self.ChildActors`)
    (if (!= _array_element Component)
      (`ActorComponent.K2_DestroyComponent` _array_element)
      (else
        (set `self.ChosenActor` _array_element)))))

(fn `SetArrayElements`
  (`KismetArrayLibrary.Array_Set` (`self.ChildActors`) 0 (`self.AssultRifle_BP`) true)
  (`KismetArrayLibrary.Array_Set` (`self.ChildActors`) 1 (`self.Shotgun_BP`) true)
  (`KismetArrayLibrary.Array_Set` (`self.ChildActors`) 2 (`self.health`) true)
  (`KismetArrayLibrary.Array_Set` (`self.ChildActors`) 3 (`self.RifleAmmo`) true)
  (`KismetArrayLibrary.Array_Set` (`self.ChildActors`) 4 (`self.ShotgunAmmo`) true))

(fn `UserConstructionScript`
  (`self.SetArrayElements`)
  (switch `/Game/Multiplayer/Blueprints/Objects/SpawnType_Enum` (`self.SpawnType`)
    (:`NewEnumerator0`
      (`self.RemoveOtherComponents` (`self.health`)))
    (:`NewEnumerator1`
      (`self.RemoveOtherComponents` (`self.AssultRifle_BP`)))
    (:`NewEnumerator4`
      (`self.RemoveOtherComponents` (`self.RifleAmmo`)))
    (:`NewEnumerator2`
      (`self.RemoveOtherComponents` (`self.Shotgun_BP`)))
    (:`NewEnumerator3`
      (`self.RemoveOtherComponents` (`self.ShotgunAmmo`)))))