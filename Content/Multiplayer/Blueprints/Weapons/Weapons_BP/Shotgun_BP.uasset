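; Shotgun weapon Blueprint that extends a parent's fire event with ammo, cooldown, sound and recoil for player 0's character.
; FIreShotgun checks magazine and CanFire, then loops per burst count, calling the parent, triggering character shooting and recoil, and decrementing ammo.
; A looping timer steps recoil back until a Delay clears it, while another Delay re-enables firing.
; An empty magazine triggers a reload message through a DoOnce, which each shot resets.
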(event `Reverse Recoil`
  (`/Game/Multiplayer/Blueprints/PlayersCharacter/PB_PlayerCharacter.Recoil Shotgun Reverse` (stale `self.FIreShotgun` _aspb_player_character))
  (`KismetSystemLibrary.Delay` 0.2)
  (`KismetSystemLibrary.K2_ClearAndInvalidateTimerHandle` (stale `self.FIreShotgun` _returnvalue)))

(event `self.FIreShotgun`
  (if (!= (`self.Shotgun_Current_mag`) 0)
    (if (`self.CanFire`)
      (set `self.CanFire` false)
      (for _ (range 1 (+ (`self.Shotgun_Burst`) 1))
        (`parent.FIreShotgun`)
        (`GameplayStatics.PlaySound2D` "/Game/Multiplayer/Blueprints/Weapons/WeaponsMesh/Sounds/Wavs/PB_Shoot.PB_Shoot" 1.0 1.0 0.0 null null)
        (bind _aspb_player_character (cast `/Game/Multiplayer/Blueprints/PlayersCharacter/PB_PlayerCharacter` (`GameplayStatics.GetPlayerPawn` 0)))
        (`/Game/Multiplayer/Blueprints/PlayersCharacter/PB_PlayerCharacter.ShotgunShooting` _aspb_player_character)
        (`/Game/Multiplayer/Blueprints/PlayersCharacter/PB_PlayerCharacter.Recoil Shotgun` _aspb_player_character)
        (bind _returnvalue (`KismetSystemLibrary.K2_SetTimerDelegate` (delegate `Reverse Recoil`) 0.025 true))
        (set `self.Shotgun_Current_mag` (- (`self.Shotgun_Current_mag`) 1))
        (`self.Reset`)
        (`KismetSystemLibrary.Delay` 1.0)
        (set `self.CanFire` true)))
    (else
      (`/Engine/EditorBlueprintResources/StandardMacros.DoOnce` false :!label _label
        (:`Completed`
          (message `/Game/Multiplayer/Blueprints/Interfaces/Reload_Shotgun.Reload_Shotgun` (`GameplayStatics.GetPlayerPawn` 0)))))))

(event `Reset`
  (goto _label :!via `Reset`))

(fn `UserConstructionScript`
  (`parent.UserConstructionScript`))