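; Base AI enemy character with Assult (shotgun) and Cover (rifle) classes, whose weapon and body color are set at construction.
; It steps a patrol target along a spline until sight, sound or damage triggers combat and timer-driven aiming.
; Timers fire randomly offset projectile bursts, while Cover enemies trace for cover every tick.
; Damage ignores other AI by display name, rolls crits, and on death ragdolls, spawning a key marker for carriers.
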(event `LookAtPlayer`
  ;[0.3811 0.5218 1] Aim At Player
  (set `self.EnemyPitch` (`KismetMathLibrary.ClampAngle` (.pitch (`KismetMathLibrary.RInterpTo` (`KismetMathLibrary.MakeRotator` 0.0 (`self.EnemyPitch`) (`self.EnemyYaw`)) (`KismetMathLibrary.NormalizedDeltaRotator` (`KismetMathLibrary.FindLookAtRotation` (`SceneComponent.GetSocketLocation` (`self.Mesh`) "hand_r") (`SceneComponent.GetSocketLocation` (`Character.Mesh` (`self.PlayerCharacter`)) "spine_03")) (`self.K2_GetActorRotation`)) (`self.DeltaSeconds`) 10.0)) -90.0 90.0))
  (set `self.EnemyYaw` (`KismetMathLibrary.ClampAngle` (.yaw (`KismetMathLibrary.RInterpTo` (`KismetMathLibrary.MakeRotator` 0.0 (`self.EnemyPitch`) (`self.EnemyYaw`)) (`KismetMathLibrary.NormalizedDeltaRotator` (`KismetMathLibrary.FindLookAtRotation` (`SceneComponent.GetSocketLocation` (`self.Mesh`) "hand_r") (`SceneComponent.GetSocketLocation` (`Character.Mesh` (`self.PlayerCharacter`)) "spine_03")) (`self.K2_GetActorRotation`)) (`self.DeltaSeconds`) 10.0)) -179.0 180.0)))

(event `self.ReceiveBeginPlay`
  (bind _spline_ref (`self.Spline_Ref`))
  ;[0.3666 0.6168 1] Event Begin Play (Set health/waypoints)
  (set `self.CurrentHealth` (`self.MaxHealth`))
  (`/Engine/EditorBlueprintResources/StandardMacros.IsValid` _spline_ref
    (:`Is Valid`
      (for _index (range (+ (`SplineComponent.GetNumberOfSplinePoints` (`/Game/Multiplayer/Blueprints/AI/Waypoint/Waypoint_BP.Spline` _spline_ref)) 1))
        (`KismetArrayLibrary.Array_Set` (`self.Spline Locations`) _index (`SplineComponent.GetLocationAtSplinePoint` (`/Game/Multiplayer/Blueprints/AI/Waypoint/Waypoint_BP.Spline` _spline_ref) _index "World") true))
      (`KismetSystemLibrary.K2_SetTimer` null "SetDesiredLocation" 0.1 true))))

(event `FireWeapon`
  ;[0.1938 0.3751 0.68] Fire Diffrent Weapon Per Class
  (if (not (`self.IsDead`))
    (switch `/Game/Multiplayer/Blueprints/AI/BehaviorTree/CombatType_ENUM` (`self.CombatType`)
      (:`NewEnumerator0`
        (`self.FireShotGun`))
      (:`NewEnumerator1`
        (`self.FireRifle`)))))

(event `SetDesiredLocation`
  (bind _current_location_index (`self.Current Location Index`))
  ;[0.4825 0.6541 1] Spline Patrol
  (set `self.DesiredLocation` (`|GetArrayItem` (`self.Spline Locations`) (`self.Current Location Index`)))
  (if (== (`self.K2_GetActorLocation`) (`self.DesiredLocation`) :`ErrorTolerance` 1500.0)
    (set `self.Current Location Index` (`KismetMathLibrary.SelectInt` (- (`self.Current Location Index`) 1) (+ (`self.Current Location Index`) 1) (`self.MinusState`)))
    (if (== (`SplineComponent.GetNumberOfSplinePoints` (`/Game/Multiplayer/Blueprints/AI/Waypoint/Waypoint_BP.Spline` (`self.Spline_Ref`))) _current_location_index)
      (set `self.MinusState` true)
      (elif (== _current_location_index 0)
        (set `self.MinusState` false)))))

(event `FireShotGun`
  ;[0.3979 0.6978 1] Fire ShotGun
  (`self.ShotGun Burst`)
  (bind _returnvalue (`KismetSystemLibrary.K2_SetTimerDelegate` (delegate `ShotGun Burst`) 1.0 true))
  (set `self.TimerHandle` _returnvalue))

(event `self.PawnSensing.OnSeePawn`
  (params (Pawn :type "Pawn Object Reference"))
  ;[0.4547 0.577 1] On Pawn Hear/sense Set combat mode
  (if (`|EnumInequality` (`self.CombatStatus`) "NewEnumerator2")
    (`self.SetCombatMode` Pawn)
    (`KismetSystemLibrary.K2_SetTimerDelegate` (delegate `LookAtPlayer`) 0.01 true :!label _label)))

(event `self.PawnSensing.OnHearNoise`
  (params (Instigator :type "Pawn Object Reference") (Location :type "Vector Structure (by ref)") (Volume :type "Float (single-precision)"))
  ;[0.4547 0.577 1] On Pawn Hear/sense Set combat mode
  (`self.SetCombatMode` Instigator)
  (goto _label))

(event `ShotGun Burst`
  (bind _returnvalue (`KismetMathLibrary.Conv_IntToDouble` (`self.ShoutGunBurstCount`)))
  ;[0.3153 0.621 1] Shotgun Burst
  (if (< (`self.FireCount`) 3)
    (`GameplayStatics.PlaySound2D` "/Game/Multiplayer/Blueprints/Weapons/WeaponsMesh/Sounds/Wavs/PB_Shoot.PB_Shoot" 1.0 1.0 0.0 null null)
    (for _ (range 1 (+ (`self.ShoutGunBurstCount`) 1))
      (bind _projectilespawninfo (`self.CalculateProjectileInfo`))
      (bind _returnvalue_2 (`|SpawnActorFromClass` "/Game/Multiplayer/Blueprints/Weapons/Projectiles/Proj_shotgun_BP.Proj_shotgun_BP_C" _projectilespawninfo "AlwaysSpawn" "OverrideRootScale" null self))
      (`/Game/Multiplayer/Blueprints/Weapons/Projectiles/Base_Projectile_BP.SetDamageInfo` _returnvalue_2 (/ (`self.DamageMin`) _returnvalue) (/ (`self.DamageMax`) _returnvalue) 0.0 0.0))
    (set `self.FireCount` (+ (`self.FireCount`) 1))
    (else
      (`KismetSystemLibrary.Delay` 1.7)
      (set `self.FireCount` 0))))

(event `/Game/Multiplayer/Blueprints/Interfaces/Cover_Interface.IsCoverAvaliable`
  (params (CoverRotation :type "Rotator Structure"))
  ;[0.3953 0.5746 1] Cover Events From Cover Object
  (set `self.CoverRotation` CoverRotation))

(event `HitReact`
  ;[0.5144 0.7136 1] Hit Reaction Event
  (`self.Hit React`))

(event `HealthBarUI`
  ;[0.3615 0.6415 1] HP UI
  (`KismetSystemLibrary.K2_SetTimerDelegate` (delegate `HealthBarUI`) 0.1 true))

(event `self.ReceiveTick`
  (params (DeltaSeconds :type "Float (single-precision)"))
  ;[0.4238 0.6101 1] Cover Mechanics Work Only On Cover AI
  (set `self.DeltaSeconds` DeltaSeconds)
  (if (`|EnumEquality` (`self.CombatType`) "NewEnumerator1")
    (`self.CoverLineTracesAI`
      (:`Output`
        (`self.CheckPlayerLocation/BlockCoverMovement`)))))

(event `FireRifle`
  ;[0.4597 0.6939 1] Fire Rifle
  (if (not (`self.IsFiring?`))
    (set `self.IsAiming` true)
    (set `self.IsFiring?` true)
    (`KismetSystemLibrary.Delay` 1.3)
    (if (`self.IsFiring?`)
      (set `self.RifleBurstCount` (`KismetMathLibrary.RandomIntegerInRange` 5 10))
      (`self.Rifle_Burst`)
      (bind _returnvalue (`KismetSystemLibrary.K2_SetTimerDelegate` (delegate `Rifle_Burst`) 0.233 true))
      (set `self.TimerHandle` _returnvalue))))

(event `/Game/Multiplayer/Blueprints/Interfaces/DamageInterface.TakeDamage`
  (params (DamageMin :type "Float (single-precision)") (DamageMax :type "Float (single-precision)") (CritChance :type "Float (single-precision)") (HitBoneName :type Name) (DamageIntagtor :type "Actor Object Reference") (ImpactVector :type "Vector Structure"))
  (bind _mesh (`self.Mesh`))
  (bind _mesh_2 (`self.Mesh`))
  ;[0.4598 0.6442 1] Calculate Damage
  (if (not (`self.NotAnotherAI` DamageIntagtor))
    (`|ExecutionSequence`
      (:`then_0`
        ;[0.4937 0.6909 1] Set Combat Mode If The AI Got Hit
        (`self.SetCombatMode` DamageIntagtor)
        ;[0.5943 0.8026 1] Hit React
        (`self.HitReact`)
        (goto _label))
      (:`then_1`
        (`self.CalculateHealth` DamageMin DamageMax CritChance HitBoneName)
        ;[0.4828 0.7041 1] Is Dead If Dead Stop Movement And Stop Firing Weapon
        (if (`self.IsDead`)
          (`self.StopFireWeapon`)
          (`MovementComponent.StopMovementImmediately` (`self.CharacterMovement`))
          ;[0.45 0.658 1] Ragdoll When Dead
          (`SkeletalMeshComponent.SetAllBodiesSimulatePhysics` _mesh true)
          (`PrimitiveComponent.AddImpulseAtLocation` _mesh ImpactVector (0.0 0.0 0.0) HitBoneName)
          (`PrimitiveComponent.SetCollisionEnabled` (`self.CapsuleComponent`) "NoCollision")
          (if (`self.CarryingKey?`)
            (`KismetSystemLibrary.Delay` 1.0)
            (`PrimitiveComponent.SetCollisionResponseToChannel` _mesh_2 "ECC_GameTraceChannel1" "ECR_Overlap")
            (bind _returnvalue (`|SpawnActorFromClass` "/Game/Multiplayer/Blueprints/Objects/KeyReflection.KeyReflection_C" (`KismetMathLibrary.MakeTransform` (`SceneComponent.GetSocketLocation` _mesh_2 "spine_01") (struct) (0.5 0.5 200.0)) "AlwaysSpawn" "OverrideRootScale" null null))
            (set `self.KeyReflectionActor` _returnvalue)
            (else
              (`KismetSystemLibrary.Delay` 5.0)
              (`self.K2_DestroyActor`))))))))

(event `StopFireWeapon`
  ;[0.5345 0.6861 1] Event Stop Firing the weapon
  (`KismetSystemLibrary.K2_ClearAndInvalidateTimerHandle` (`self.TimerHandle`))
  (set `self.IsAiming` false)
  (set `self.IsFiring?` false)
  (set `self.FireCount` 0))

(event `Rifle_Burst`
  ;[0.4031 0.709 1] Rifle Burst
  (if (< (`self.FireCount`) (`self.RifleBurstCount`))
    (`GameplayStatics.PlaySound2D` "/Game/Multiplayer/Blueprints/Weapons/WeaponsMesh/Sounds/Wavs/PB_Shoot.PB_Shoot" 1.0 1.0 0.0 null null)
    (bind _projectilespawninfo (`self.CalculateProjectileInfo`))
    (bind _returnvalue (`|SpawnActorFromClass` "/Game/Multiplayer/Blueprints/Weapons/Projectiles/Proj_Assult_BP.Proj_Assult_BP_C" _projectilespawninfo "AlwaysSpawn" "OverrideRootScale" null self))
    (`/Game/Multiplayer/Blueprints/Weapons/Projectiles/Base_Projectile_BP.SetDamageInfo` _returnvalue (`self.DamageMin`) (`self.DamageMax`) 0.0 0.0)
    (set `self.FireCount` (+ (`self.FireCount`) 1))))

(fn `CalculateHealth`
  (params (MinDamage :type "Float (double-precision)") (MaxDamage :type "Float (double-precision)") (CritChance :type "Float (double-precision)") (HitBoneName :type Name))
  (locals (LocalDamage :type "Float (double-precision)" :default 0.0))
  ;[1 1 1] Check To See Player Not Dead
  (if (not (`self.IsDead`))
    ;[1 1 1] Set Local Damage
    (set `local.LocalDamage` (`KismetMathLibrary.Conv_IntToDouble` (`KismetMathLibrary.Round` (`KismetMathLibrary.RandomFloatInRange` MinDamage MaxDamage))))
    (`|ExecutionSequence`
      (:`then_0`
        ;[1 1 1] Set Crit Chance Damage
        (if (<= (`KismetMathLibrary.RandomFloatInRange` 0.0 100.0) CritChance)
          (set `local.LocalDamage` (* (`local.LocalDamage`) 3.0))))
      (:`then_1`
        ;[1 1 1] Set HeadShot Damage
        (switch `name` HitBoneName
          (:`head`
            (set `local.LocalDamage` (* (`local.LocalDamage`) 3.0)))))
      (:`then_2`
        ;[1 1 1] Set Health to 0 And Set isDead If Hp Reachs 0 or Below
        (bind _output_get (set `self.CurrentHealth` (- (`self.CurrentHealth`) (`local.LocalDamage`))))
        (if (<= _output_get 0.0)
          (set `self.CurrentHealth` 0.0)
          (set `self.IsDead` true))))))

(fn `CalculateProjectileInfo`
  (returns (ProjectileSpawnInfo :type "Transform Structure"))
  (bind _returnvalue (`SceneComponent.K2_GetComponentLocation` (`self.MuzzleArrow`)))
  (bind _x (.x _returnvalue))
  (bind _y (.y _returnvalue))
  (bind _z (.z _returnvalue))
  (bind (_returnvalue3 _returnvalue2 _returnvalue_2) (`self.RandomizeProjectileBullets` _x _x _y _z _y _z))
  (return (`KismetMathLibrary.MakeTransform` (`KismetMathLibrary.MakeVector` _returnvalue3 _returnvalue2 _returnvalue_2) (`KismetMathLibrary.FindLookAtRotation` _returnvalue (`SceneComponent.GetSocketLocation` (`Character.Mesh` (`self.PlayerCharacter`)) "spine_02")) (1.0 1.0 1.0))))

(fn `NotAnotherAI`
  (params (Object :type "Object Object Reference"))
  (returns (ReturnValue :type Boolean))
  (return (`KismetStringLibrary.EqualEqual_StrStr` (`KismetStringLibrary.Split` (`KismetSystemLibrary.GetDisplayName` Object) "_") "BaseEnemyCharacter")))

(fn `RandomizeProjectileBullets`
  (params (A1 :type "Float (double-precision)") (A2 :type "Float (double-precision)") (A3 :type "Float (double-precision)") (A4 :type "Float (double-precision)") (A5 :type "Float (double-precision)") (A6 :type "Float (double-precision)"))
  (returns (ReturnValue3 :type "Float (double-precision)") (ReturnValue2 :type "Float (double-precision)") (ReturnValue :type "Float (double-precision)"))
  (return (`KismetMathLibrary.RandomFloatInRange` (- A1 10.0) (+ A2 10.0)) (`KismetMathLibrary.RandomFloatInRange` (- A5 10.0) (+ A3 10.0)) (`KismetMathLibrary.RandomFloatInRange` (- A6 10.0) (+ A4 10.0))))

(fn `SetCombatMode`
  (params (`Sensed Pawn` :type "Object Object Reference"))
  (if (not (`|EnumEquality` (`self.CombatStatus`) "NewEnumerator2"))
    (bind _aspb_player_character (cast `/Game/Multiplayer/Blueprints/PlayersCharacter/PB_PlayerCharacter` `Sensed Pawn`)
      (:`then`
        (set `self.PlayerCharacter` _aspb_player_character)
        (set `self.CombatStatus` "NewEnumerator2"))
      (:`CastFailed`
        (`KismetSystemLibrary.PrintString` "Cast Failed : BaseEnemyCharacter_BP Cast to PB_PlayerCharacter Set Combat")))
    (else
      (bind _aspb_player_character_2 (cast `/Game/Multiplayer/Blueprints/PlayersCharacter/PB_PlayerCharacter` `Sensed Pawn`))
      (set `self.PlayerCharacter` _aspb_player_character_2))))

(fn `SetIsTakingCover`
  (params (IsTakingCover :type Boolean))
  (bind _output_get (set `self.IsTakingCover` IsTakingCover))
  (if _output_get
    ;[1 1 1] If Taking Cover Set Actor Rotation To Cover Rotation
    (`self.K2_SetActorRotation` (`self.CoverRotation`))
    (else
      ;[1 1 1] If Not In Cover Unset Cover Go Left/Right
      (set `self.CoverGoLeft` false)
      (set `self.CoverGoRight` false))))

(fn `UserConstructionScript`
  (bind _ai_weapon (`self.AI_Weapon`))
  (`|ExecutionSequence`
    (:`then_0`
      ;[1 1 1] Change Char Weapon Per Class
      (switch `/Game/Multiplayer/Blueprints/AI/BehaviorTree/CombatType_ENUM` (`self.CombatType`)
        (:`NewEnumerator0`
          (`SkinnedMeshComponent.SetSkinnedAssetAndUpdate` _ai_weapon "/Game/Multiplayer/Blueprints/Weapons/WeaponsMesh/Launcher.Launcher" true)
          (bind _returnvalue (`PrimitiveComponent.CreateDynamicMaterialInstance` (`self.Mesh`) 0 "/Game/Multiplayer/Characters/UE4_Mannequin/Materials/M_UE4Man_Body.M_UE4Man_Body" "None"))
          (`MaterialInstanceDynamic.SetVectorParameterValue` _returnvalue "BodyColor" (struct :`R` 0.14 :`G` 0.003662 :`A` 1.0)))
        (:`NewEnumerator1`
          (`SkinnedMeshComponent.SetSkinnedAssetAndUpdate` _ai_weapon "/Game/Multiplayer/Blueprints/Weapons/WeaponsMesh/Rifle.Rifle" true)
          (bind _returnvalue_2 (`PrimitiveComponent.CreateDynamicMaterialInstance` (`self.Mesh`) 0 "/Game/Multiplayer/Characters/UE4_Mannequin/Materials/M_UE4Man_Body.M_UE4Man_Body" "None"))
          (`MaterialInstanceDynamic.SetVectorParameterValue` _returnvalue_2 "BodyColor" (struct :`R` 0.000121 :`G` 0.09 :`A` 1.0)))))
    (:`then_1`
      ;[1 1 1] Attach Weapon To Mesh
      (`SceneComponent.K2_AttachTo` (`self.AI_Weapon`) (`self.Mesh`) "AIWeaponSocket" "SnapToTarget" true))
    (:`then_2`
      ;[1 1 1] Attach Muzzle Arrow To Muzzle Socket On The Weapon
      (`SceneComponent.K2_AttachTo` (`self.MuzzleArrow`) (`self.AI_Weapon`) (`self.Muzzle`) "SnapToTarget" true))
    (:`then_3`
      (switch `/Game/Multiplayer/Blueprints/AI/BehaviorTree/CombatStatus_ENUM` (`self.CombatStatus`)
        (:`NewEnumerator0`
          (switch `/Game/Multiplayer/Blueprints/AI/BehaviorTree/CombatType_ENUM` (`self.CombatType`)
            (:`NewEnumerator1`
              (bind _returnvalue_3 (`PrimitiveComponent.CreateDynamicMaterialInstance` (`self.Mesh`) 0 "/Game/Multiplayer/Characters/UE4_Mannequin/Materials/M_UE4Man_Body.M_UE4Man_Body" "None"))
              (`MaterialInstanceDynamic.SetVectorParameterValue` _returnvalue_3 "BodyColor" (struct :`A` 1.0)))))))
    (:`then_4`
      ;[1 1 1] Set WayPoints
      (if (`self.CarryingKey?`)
        (bind _returnvalue_4 (`PrimitiveComponent.CreateDynamicMaterialInstance` (`self.Mesh`) 0 "/Game/Multiplayer/Characters/UE4_Mannequin/Materials/M_UE4Man_Body.M_UE4Man_Body" "None"))
        (`MaterialInstanceDynamic.SetVectorParameterValue` _returnvalue_4 "BodyColor" (struct :`R` 0.24 :`G` 0.196666 :`A` 1.0))))))